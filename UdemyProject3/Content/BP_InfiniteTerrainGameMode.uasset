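; Game mode for an infinite-terrain game that spawns the world tile by tile and tracks how many tiles are conquered.
; At BeginPlay it populates a pool of nav mesh bounds volumes, then spawns three starting tiles.
; Each new BP_Tile receives that pool and returns its attach location, which becomes the transform for the next tile, forming a chain.
; Conquering a tile increments Score and prints it.
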(event `self.ReceiveBeginPlay`
  (`self.PopulateBoundsVolumePool`)
  (for _ (range 3)
    (`self.Spawn Tile`)))

(fn `NewTileConquered`
  (bind _result (`/Engine/EditorBlueprintResources/StandardMacros.IncrementInt` (`self.Score`))
    (:`  `
      (`KismetSystemLibrary.PrintString` (`KismetStringLibrary.Conv_IntToString` _result)))))

(fn `Spawn Tile`
  (bind _returnvalue (`|SpawnActorFromClass` "/Game/Terrain/BP_Tile.BP_Tile_C" (`self.NextTileTransform`) "Undefined" "OverrideRootScale" null null))
  (`Tile.SetPool` _returnvalue (`self.NavMeshBoundsVolumePool`))
  (bind _attachtransform (`/Game/Terrain/BP_Tile.GetAttachLocation` _returnvalue))
  (set `self.NextTileTransform` _attachtransform))

(fn `UserConstructionScript`)