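; Terrain tile for an infinite-terrain mode that fills itself on BeginPlay with randomly placed props and AI characters.
; Its barrier starts locked, turning passable and green while the player overlaps the locking volume, then solid and red again on exit.
; When the player enters the destroy volume, the tile asks the game mode to spawn another and destroys itself.
; An arrow component supplies the attach transform for chaining tiles.
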(event `self.ReceiveBeginPlay`
  (`self.Lock`)
  (`self.SpawnProps`)
  (`self.PlaceAIPawns` "/Game/Character/Blueprints/BP_Character.BP_Character_C" 2 4 100.0))

(event `self.LockingVolume.OnComponentBeginOverlap`
  (params (OverlappedComponent :type "PrimitiveComponent Object Reference") (OtherActor :type "Actor Object Reference") (OtherComp :type "PrimitiveComponent Object Reference") (OtherBodyIndex :type Integer) (bFromSweep :type Boolean) (SweepResult :type "HitResult Structure (by ref)"))
  (`self.IsPlayer` OtherActor)
  (`self.Unlock`))

(event `self.LockingVolume.OnComponentEndOverlap`
  (params (OverlappedComponent :type "PrimitiveComponent Object Reference") (OtherActor :type "Actor Object Reference") (OtherComp :type "PrimitiveComponent Object Reference") (OtherBodyIndex :type Integer))
  (`self.IsPlayer` OtherActor)
  (`self.Lock`))

(event `self.DestroyVolume.OnComponentBeginOverlap`
  (params (OverlappedComponent :type "PrimitiveComponent Object Reference") (OtherActor :type "Actor Object Reference") (OtherComp :type "PrimitiveComponent Object Reference") (OtherBodyIndex :type Integer) (bFromSweep :type Boolean) (SweepResult :type "HitResult Structure (by ref)"))
  (`self.IsPlayer` OtherActor)
  (`self.SpawnNextTile`)
  (`self.K2_DestroyActor`))

(fn `GetAttachLocation`
  (returns (AttachTransform :type "Transform Structure"))
  (return (`SceneComponent.K2_GetComponentToWorld` (`self.Arrow`))))

(fn `Lock`
  (`PrimitiveComponent.SetCollisionEnabled` (`self.Barrier`) "QueryAndPhysics")
  (`PrimitiveComponent.SetMaterial` (`self.Barrier`) 0 "/Game/Terrain/MI_Barrier_Red.MI_Barrier_Red"))

(fn `SpawnNextTile`
  (bind _asbp_infinite_terrain_game_mode (cast `/Game/BP_InfiniteTerrainGameMode` (`GameplayStatics.GetGameMode`)))
  (`/Game/BP_InfiniteTerrainGameMode.Spawn Tile` _asbp_infinite_terrain_game_mode))

(fn `SpawnProps`
  (`|ExecutionSequence`
    (:`then_0`
      (`self.PlaceActors` "/Game/Props/Blueprints/BP_Barrel.BP_Barrel_C" 0 3 100.0 1.0 1.2)
      (`self.PlaceActors` "/Game/Props/Blueprints/BP_Barrels.BP_Barrels_C" 0 2 200.0 1.0 1.2)
      (`self.PlaceActors` "/Game/Props/Blueprints/BP_TrafficBarrel.BP_TrafficBarrel_C" 0 3 100.0))
    (:`then_1`
      (`self.PlaceActors` "/Game/Props/Blueprints/BP_Box2.BP_Box2_C" 0 3 150.0 1.0 1.5)
      (`self.PlaceActors` "/Game/Props/Blueprints/BP_Box1.BP_Box1_C" 0 3 200.0 1.0 1.5)
      (`self.PlaceActors` "/Game/Props/Blueprints/BP_Boxes.BP_Boxes_C" 0 2))
    (:`then_2`
      (`self.PlaceActors` "/Game/Props/Blueprints/BP_CartonGarbage.BP_CartonGarbage_C" 0 2 150.0 1.0 1.2)
      (`self.PlaceActors` "/Game/Props/Blueprints/BP_Hose.BP_Hose_C" 0 3 50.0 1.0 3.0)
      (`self.PlaceActors` "/Game/Props/Blueprints/BP_WaterTank.BP_WaterTank_C" 0 2 200.0 1.0 1.2))))

(fn `Unlock`
  (`PrimitiveComponent.SetCollisionEnabled` (`self.Barrier`) "NoCollision")
  (`PrimitiveComponent.SetMaterial` (`self.Barrier`) 0 "/Game/Terrain/MI_Barrier_Green.MI_Barrier_Green"))

(fn `UserConstructionScript`)